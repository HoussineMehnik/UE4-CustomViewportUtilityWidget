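; BP_SceneCaptureActor is a scene capture actor that renders only on demand through its SceneCaptureComponent2D.
; Init turns off capture every frame and on movement, leaving captures to explicit calls.
; Update moves the actor to a given location and rotation and captures immediately, while RefreshCapture re-captures in place.
; Separate events hide a given component from the capture or clear the hidden component list.
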(event `Init`
  (bind _scenecapturecomponent2d (`self.SceneCaptureComponent2D`))
  (set `SceneCaptureComponent.bCaptureEveryFrame` false _scenecapturecomponent2d)
  (set `SceneCaptureComponent.bCaptureOnMovement` false _scenecapturecomponent2d))

(event `Update`
  (params (Location :type "Vector Structure") (Rotation :type "Rotator Structure"))
  (`self.K2_SetActorLocationAndRotation` Location Rotation)
  (`SceneCaptureComponent2D.CaptureScene` (`self.SceneCaptureComponent2D`)))

(event `Refresh Capture`
  (`SceneCaptureComponent2D.CaptureScene` (`self.SceneCaptureComponent2D`)))

(event `Hide Component`
  (params (InComponent :type "PrimitiveComponent Object Reference"))
  (`SceneCaptureComponent.HideComponent` (`self.SceneCaptureComponent2D`) InComponent))

(event `Reset Hidden Components List`
  (`SceneCaptureComponent.ClearHiddenComponents` (`self.SceneCaptureComponent2D`)))

(fn `UserConstructionScript`)